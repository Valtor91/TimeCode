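; GM_Game is the game mode that keeps a list of connected player controllers for a multiplayer game.
; PostLogin adds each controller uniquely and OnLogout removes it.
; After a retriggerable delay, PostLogin checks for three players, but that branch does nothing.
; A disconnected block, which never runs, would compare player count to session connection settings, kick surplus players and update the session.
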(event `self.K2_PostLogin`
  (params (NewPlayer :type "PlayerController Object Reference"))
  (`KismetArrayLibrary.Array_AddUnique` (`self.PlayerControleur`) NewPlayer)
  (`KismetSystemLibrary.RetriggerableDelay` 2.0)
  (if (== (`KismetArrayLibrary.Array_Length` (`GameStateBase.PlayerArray` (`GameplayStatics.GetGameState`))) 3)
    _))

(event `self.K2_OnLogout`
  (params (ExitingController :type "Controller Object Reference"))
  (bind _asplayer_controller (cast `PlayerController` ExitingController))
  (`KismetArrayLibrary.Array_RemoveItem` (`self.PlayerControleur`) _asplayer_controller))

(fn `UserConstructionScript`)